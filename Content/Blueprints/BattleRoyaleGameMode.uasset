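; Game mode for a cowboy battle royale that tracks joined players and declares the last one standing as winner.
; PostLogin counts and stores each new controller, and PlayerDie decrements that count.
; When one player remains, it waits briefly, takes the first Cowboy_character found in the world, and sends its username to ShowWinner on every stored CowboyController.
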(event Custom|ShowWinner
  (params (InText :type Text))
  (for _array_element (Variables|Default|GetNew%20Player)
    (bind _ascowboy_controller (Utilities|Casting|CastToCowboyController _array_element))
    (Default|ShowWinner _ascowboy_controller InText)))

(event EventBeginPlay)

(event EventTick
  (params (DeltaSeconds :type Float%20%28single-precision%29)))

(event EventPostLogin
  (params (NewPlayer :type Player%20Controller%20Object%20Reference))
  (Variables|Default|SetNumPlayers (+ (Variables|Default|GetNumPlayers) 1))
  (Utilities|Array|Add (Variables|Default|GetNew%20Player) NewPlayer))

(event EventPlayerDie
  (params (Username :type String))
  (Development|PrintString Username)
  (bind _output_get (Variables|Default|SetNumPlayers (- (Variables|Default|GetNumPlayers) 1)))
  (if (== _output_get 1)
    (Utilities|FlowControl|Delay 1.0)
    (bind _outactors (Actor|GetAllActorsOfClass "/Game/CharacterActors/ThirdPersonBP/Blueprints/Cowboy_character.Cowboy_character_C"))
    (Development|PrintString (Variables|/Game/CharacterActors/ThirdPersonBP/Blueprints/Cowboy_character.Cowboy_character_C|GetUsername (Utilities|Array|Get(acopy) _outactors)) true true "(R=1.000000,G=0.118821,B=0.218526,A=1.000000)")
    (CallFunction|ShowWinner (Utilities|Text|ToText(String) (Variables|/Game/CharacterActors/ThirdPersonBP/Blueprints/Cowboy_character.Cowboy_character_C|GetUsername (Utilities|Array|Get(acopy) _outactors))))))

(fn ConstructionScript)