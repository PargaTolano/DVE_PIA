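; TracerRound_BP is a tracer round actor that damages what it overlaps and removes itself on impact.
; Sphere overlaps send a CharacterDamageMessage with a fixed amount to the other actor, then destroy the round after a short delay.
; Sphere hits destroy the round immediately without sending damage.
; Both events skip the actor stored in Ignore and other tracer rounds.
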(event OnComponentHit(Sphere)
  (params (HitComponent :type Primitive%20Component%20Object%20Reference) (OtherActor :type Actor%20Object%20Reference) (OtherComp :type Primitive%20Component%20Object%20Reference) (NormalImpulse :type Vector :default "0, 0, 0") (Hit :type Hit%20Result%20Structure%20%28by%20ref%29))
  (if (and (!= OtherActor (Variables|Default|GetIgnore)) (!= (Utilities|GetClass OtherActor) "TracerRound_BP_C"))
    (Actor|DestroyActor)))

(event OnComponentBeginOverlap(Sphere)
  (params (OverlappedComponent :type Primitive%20Component%20Object%20Reference) (OtherActor :type Actor%20Object%20Reference) (OtherComp :type Primitive%20Component%20Object%20Reference) (OtherBodyIndex :type Integer) (bFromSweep :type Boolean) (SweepResult :type Hit%20Result%20Structure%20%28by%20ref%29))
  (if (and (!= (Variables|Default|GetIgnore) OtherActor) (!= (Utilities|GetClass OtherActor) "TracerRound_BP_C"))
    (Class|BPICharacter|CharacterDamage(Message) OtherActor 15)
    (Utilities|FlowControl|Delay 0.2)
    (Actor|DestroyActor)))

(fn ConstructionScript)